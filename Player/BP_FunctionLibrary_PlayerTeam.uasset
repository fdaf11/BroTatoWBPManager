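; Blueprint function library that classifies a given player state by its team relation to the local client's player.
; IsSameTeamInClient compares the input against LocalPS from the BTUI controller, then calls that player state's IsSameTeam.
; It returns one of three enum values: the local player itself, a teammate, or neither.
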(fn `IsSameTeamInClient`
  (params (InPS1 :type "BTPlayerState Object Reference"))
  (returns (ReturnValue :type "/Game/UI/Layout/Player/E_UI_PlayerTeammateType Enum"))
  (locals (InPS :type "BTPlayerState Object Reference"))
  (set `local.InPS` InPS1)
  (return (select `bool` (== (`BTUIController.LocalPS` (`BTGameplayFunctionLibrary.GetBTUIController` null)) (`local.InPS`)) :`false` (select `bool` (`BTPlayerState.IsSameTeam` (`BTUIController.LocalPS` (`BTGameplayFunctionLibrary.GetBTUIController` null)) (`local.InPS`)) :`false` "NewEnumerator2" :`true` "NewEnumerator1" :!type "/Game/UI/Layout/Player/E_UI_PlayerTeammateType Enum") :`true` "NewEnumerator0")))