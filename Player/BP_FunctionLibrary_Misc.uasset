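; BP_FunctionLibrary_Misc is a miscellaneous helper library for debug logging and skill-slot conversion.
; LogMapIntInt joins an integer map's entries into a bracketed, labelled string and logs it via MyLogDisplay, pairing every key with the first value only.
; Two converters map skill indices 0–4 to operation widget types and back, using a Select one way and a switch on the skill enum the other.
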(fn `Log Map Int Int`
  (params (LogSection :type String :default "MyLog") (InData :type "Map of Integer to Integer (by ref)") (LogPrefix :type String) (KeyName :type String) (ValueName :type String))
  (locals (L_ResStr :type String))
  ;[0.5938 0 1] 日志
  (bind _keys (`BlueprintMapLibrary.Map_Keys` InData))
  (bind _values (`BlueprintMapLibrary.Map_Values` InData))
  (for _array_element _keys
    (set `local.L_ResStr` (`MyFunctionLibrary_NormalUI.AppendStringIfNotEmpty` (`local.L_ResStr`) (`KismetTextLibrary.Conv_TextToString` (`|FormatText` "[{OneItem}], " (`MyFunctionLibrary_NormalUI.AppendStringIfNotEmpty` (`MyFunctionLibrary_NormalUI.AppendStringIfNotEmpty` KeyName (`KismetStringLibrary.Conv_IntToString` _array_element) ": ") (`MyFunctionLibrary_NormalUI.AppendStringIfNotEmpty` ValueName (`KismetStringLibrary.Conv_IntToString` (`|GetArrayItem` _values)) ": ") ", "))))))
  (`MyFunctionLibrary_UtilityTools.MyLog_Display` (`local.LogSection`) (`MyFunctionLibrary_NormalUI.AppendStringIfNotEmpty` LogPrefix (`local.L_ResStr`) ": ")))

(fn `SkillIndex2WidgetType`
  (params (Index :type Integer))
  (returns (ReturnValue :type "EOperationWidgetType Enum"))
  (return (select `int` Index :`0` "OperationWidgetType3" :`1` "OperationWidgetType4" :`2` "OperationWidgetType5" :`3` "OperationWidgetType6" :`4` "OperationWidgetType7" :!type "EOperationWidgetType Enum")))

(fn `WidgetTypeTrans2SkillIndex`
  (params (Type :type "EOperationWidgetType Enum" :default "None"))
  (returns (Index :type Integer))
  (switch `EOperationWidgetType` Type
    (:`OperationWidgetType3`
      (return 0))
    (:`OperationWidgetType4`
      (return 1))
    (:`OperationWidgetType5`
      (return 2))
    (:`OperationWidgetType6`
      (return 3))
    (:`OperationWidgetType7`
      (return 4))))